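; BP_Zombie is a zombie enemy that takes point damage, tracks its Health and dies when it runs out.
; Point damage on a living zombie lowers Health, then plays a hit reaction montage on the mesh with a debug print of Health, or triggers Death at zero or below.
; Death sets IsDead so further hits are ignored, stops character movement immediately and plays the dying montage.
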(event `self.ReceivePointDamage`
  (params (Damage :type "Float (single-precision)") (DamageType :type "DamageType Object Reference") (HitLocation :type "Vector Structure") (HitNormal :type "Vector Structure") (HitComponent :type "PrimitiveComponent Object Reference") (BoneName :type Name) (ShotFromDirection :type "Vector Structure") (InstigatedBy :type "Controller Object Reference") (DamageCauser :type "Actor Object Reference") (HitInfo :type "HitResult Structure (by ref)"))
  (if (`self.IsDead?`)
    _
    (elif (<= (`self.Health`) 0.0)
      (`self.Death`)
      (else
        (set `self.Health` (- (`self.Health`) Damage))
        (if (<= (`self.Health`) 0.0)
          (`self.Death`)
          (else
            (`|PlayMontage` (`self.Mesh`) "/Game/Main/Zombie/Animations/Zombie_Reaction_Hit_mixamo_com_Montage.Zombie_Reaction_Hit_mixamo_com_Montage"
              (:`then`
                (`KismetSystemLibrary.PrintString` (`KismetStringLibrary.Concat_StrStr` "Zombie Health :" (`KismetStringLibrary.Conv_DoubleToString` (`self.Health`))))))))))))

(event `Death`
  (set `self.IsDead?` true)
  (`MovementComponent.StopMovementImmediately` (`self.CharacterMovement`))
  (`|PlayMontage` (`self.Mesh`) "/Game/Main/Zombie/Animations/zombie_dying_Montage.zombie_dying_Montage"))

(fn `UserConstructionScript`)